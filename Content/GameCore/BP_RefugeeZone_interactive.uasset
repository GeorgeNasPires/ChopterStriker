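; Refugee zone actor that sends a stream of refugees to a requested position when CallRefugees is triggered.
; Each call, while RefugeeCount is above zero, spawns a Refugee at one of three random spawn points and orders it to move to that position.
; The event re-calls itself after a short delay, decrementing the count only after that call, so each check precedes its decrement.
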(event `CallRefugees`
  (params (Position :type "Vector Structure"))
  (if (> (`self.RefugeeCount`) 0)
    (bind _returnvalue (`|SpawnActorFromClass` "/Game/Characters/Refugee/Refugee.Refugee_C" (`KismetMathLibrary.MakeTransform` (select `int` (`KismetMathLibrary.RandomIntegerInRange` 0 2) :`0` (`SceneComponent.K2_GetComponentLocation` (`self.SpawnPoint01`)) :`1` (`SceneComponent.K2_GetComponentLocation` (`self.SpawnPoint02`)) :`2` (`SceneComponent.K2_GetComponentLocation` (`self.SpawnPoint03`)))) "Undefined" "OverrideRootScale" null null))
    (`/Game/Characters/Refugee/Refugee.MoveToPosition` _returnvalue Position)
    (`KismetSystemLibrary.Delay` 2.0)
    (`self.CallRefugees` Position)
    (`/Engine/EditorBlueprintResources/StandardMacros.DecrementInt` (`self.RefugeeCount`))))

(fn `UserConstructionScript`)