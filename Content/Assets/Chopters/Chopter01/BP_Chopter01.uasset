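; Player helicopter Blueprint that handles interactions, damage and mission guidance.
; On BeginPlay it creates the HUD and attaches a spawned ladder; input or HUD button triggers interaction, lowering the ladder to terrain height at refugee zones.
; A compass, visible only while flying, points each tick to the nearest supply item when none is carried, otherwise to the next mission location.
; Damage feeds ChopterDamage, while falling and exploding events spawn ChopterExplode actors.
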(event `self.ReceiveBeginPlay`
  (bind _returnvalue (`|CreateWidget` "/Game/Assets/Chopters/ChopterUI/W_ChopterUI.W_ChopterUI_C" null self))
  (bind _output_get (set `self.UI_ref` _returnvalue))
  (add `/Game/Assets/Chopters/ChopterUI/W_ChopterUI.InteractionButtonPressed` _output_get (`|CreateDelegate` :!event `InteractionButtonClicked`))
  (`UserWidget.AddToViewport` (`self.UI_ref`) 0)
  (bind _returnvalue_2 (`|SpawnActorFromClass` "/Game/Assets/HopeLadder/ChopterLadder.ChopterLadder_C" (`KismetMathLibrary.MakeTransform` (+ (`self.K2_GetActorLocation`) (0.0 30.0 50.0))) "Undefined" "OverrideRootScale" null self null))
  (bind _output_get_2 (set `self.LadderActor` _returnvalue_2))
  (`self.K2_AttachToComponent` _output_get_2 (`self.ChopterYaw`) "None" "KeepWorld" "KeepRelative" "KeepRelative" true)
  (add `self.ED_EmbarkedRefugees` (`|CreateDelegate` :!event `ED_EmbarkedRefugees_Event`)))

(event `self.OnInteractiveItemResponse`
  (params (itemType :type "ItemTypesEnum Enum" :default "NONE"))
  (bind _output_get (set `self.InteractionItem` itemType))
  (`/Game/Assets/Chopters/ChopterUI/W_ChopterUI.Set Interactive Icon` (`self.UI_ref`) (`self.ChopterStat`) _output_get))

(event `self.OnStatChanged`
  (params (Stat :type "ChopterStats Enum" :default "OFF"))
  (bind _output_get (set `self.Stat` Stat))
  (`|ExecutionSequence`
    (:`then_0`
      (switch `ChopterStats` _output_get))
    (:`then_1`
      (`SceneComponent.SetVisibility` (`self.Compass`) (`|EnumEquality` (`self.Stat`) "FLING") false))))

(event `InputAction|InteractionButton`
  (params (Key :type "Key Structure"))
  (bind _interactionitem (`self.InteractionItem`))
  (:`Pressed`
    (`self.InteractionAction` _interactionitem :!label _label)
    (switch `ItemTypesEnum` _interactionitem
      (:`REFUGEEZONE`
        (`/Game/Assets/HopeLadder/ChopterLadder.LadderDown` (`self.LadderActor`) (`KismetMathLibrary.Vector_Distance` (`self.GetLocationInTerrain`) (`self.K2_GetActorLocation` (`self.LadderActor`))))))))

(event `InteractionButtonClicked`
  (goto _label))

(event `self.SpawnChopterFaller`
  (params (bodyRotator :type "Rotator Structure") (topRotator :type "Rotator Structure") (tailRotator :type "Rotator Structure"))
  (`/Engine/EditorBlueprintResources/StandardMacros.DoOnce` false
    (:`Completed`
      (`|SpawnActorFromClass` "/Game/Assets/Chopters/Chopter01/ChopterExplode.ChopterExplode_C" (`self.GetTransform`) "Undefined" "OverrideRootScale" null topRotator tailRotator bodyRotator false null))))

(event `self.OnChopterExplode`
  (`|SpawnActorFromClass` "/Game/Assets/Chopters/Chopter01/ChopterExplode.ChopterExplode_C" (`self.GetTransform`) "Undefined" "OverrideRootScale" null (struct) (struct) (struct) true null))

(event `self.ReceiveAnyDamage`
  (params (Damage :type "Float (single-precision)") (DamageType :type "DamageType Object Reference") (InstigatedBy :type "Controller Object Reference") (DamageCauser :type "Actor Object Reference"))
  (`self.ChopterDamage` Damage))

(event `ED_EmbarkedRefugees_Event` :!signature `self.ED_EmbarkedRefugees`
  (params (LadderPosition :type "Vector Structure")))

(event `self.ReceiveTick`
  (params (DeltaSeconds :type "Float (single-precision)"))
  (bind (_distance _returnvalue) (`GameplayStatics.FindNearestActor` (`SceneComponent.K2_GetComponentLocation` (`self.Compass`)) (`/Game/GameCore/MisionsStructures/LevelMission.GetItemMission` (`self.LevelMission`))))
  (if (`KismetArrayLibrary.Array_IsValidIndex` (`/Game/GameCore/MisionsStructures/LevelMission.GetItemMission` (`self.LevelMission`)))
    (`SceneComponent.K2_SetWorldRotation` (`self.Compass`) (`KismetMathLibrary.FindLookAtRotation` (`SceneComponent.K2_GetComponentLocation` (`self.Compass`)) (select `bool` (and (not (`self.IsCarrySupply`)) (`|EnumEquality` (`InteractiveItem.ItemType` (cast `InteractiveItem` _returnvalue :!pure true)) "SUPPLIES")) :`false` (`/Game/GameCore/MisionsStructures/LevelMission.GetNextMissionLocation` (`self.LevelMission`)) :`true` (`self.K2_GetActorLocation` _returnvalue))) false false)
    (else
      (`SceneComponent.K2_SetWorldRotation` (`self.Compass`) (`KismetMathLibrary.FindLookAtRotation` (`SceneComponent.K2_GetComponentLocation` (`self.Compass`)) (`/Game/GameCore/MisionsStructures/LevelMission.GetNextMissionLocation` (`self.LevelMission`))) false false))))

(fn `F_GetFuel`
  (returns (Fuel :type "Float (single-precision)"))
  (return (`self.Fuel`)))

(fn `F_GetLife`
  (returns (Life :type "Float (single-precision)"))
  (return (`self.Life`)))

(fn `UserConstructionScript`)